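; AI controller for the cleaning bot that starts its behavior tree and animates its head when the destination changes.
; BeginPlay sets up the Blackboard with the pawn's start location and a hardcoded destination, runs the tree and binds the destination-change dispatcher.
; Each change restarts a timeline that lerps only the head mesh's world yaw, using the look-at angle from the TargetToFollow actor to the head.
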(event Custom|Changed%20Destination
  ;[1 1 1] Head Rotation
  (if (!= (Variables|Default|GetCleaningBot) 0)
    _
    (else
      (bind _asbp_cleaning_bot (Utilities|Casting|CastToBP_CleaningBot (Pawn|GetControlledPawn)))
      (Variables|Default|SetCleaningBot _asbp_cleaning_bot)))
  (Variables|Default|SetInitialRotation (Transformation|GetWorldRotation (Variables|/Game/AI/CleaningnRobot/BP_CleaningBot.BP_CleaningBot_C|GetHeadMesh (Variables|Default|GetCleaningBot))))
  (Utilities|FlowControl|Sequence
    (:then_0
      (bind _newtrack_0 (Timeline|RotationTimeLine Stop)
        (:Update
          (Transformation|SetWorldRotation (Variables|/Game/AI/CleaningnRobot/BP_CleaningBot.BP_CleaningBot_C|GetHeadMesh (Variables|Default|GetCleaningBot)) (Math|Rotator|Lerp(Rotator) (Math|Rotator|MakeRotator (.Roll (Math|Rotator|BreakRotator (Variables|Default|GetInitialRotation))) (.Pitch (Math|Rotator|BreakRotator (Variables|Default|GetInitialRotation))) (.Yaw (Math|Rotator|BreakRotator (Variables|Default|GetInitialRotation)))) (Math|Rotator|MakeRotator (.Roll (Math|Rotator|BreakRotator (Variables|Default|GetInitialRotation))) (.Pitch (Math|Rotator|BreakRotator (Variables|Default|GetInitialRotation))) (.Yaw (Math|Rotator|BreakRotator (Math|Rotator|FindLookatRotation (Transformation|GetActorLocation (.AsActor (Utilities|Casting|CastToActor (AI|Components|Blackboard|GetValueasObject (AI|GetBlackboard self) (Variables|Default|GetTargetToFollow))))) (Transformation|GetWorldLocation (Variables|/Game/AI/CleaningnRobot/BP_CleaningBot.BP_CleaningBot_C|GetHeadMesh (Variables|Default|GetCleaningBot))))))) _newtrack_0) false false))))
    (:then_1
      (Timeline|RotationTimeLine PlayFromStart))))

(event EventBeginPlay
  (bind _self self)
  (bind _returnvalue (AI|GetBlackboard _self))
  ;[1 1 1] Initial Blackboard Setup
  (Class|AIController|UseBlackboard (AI|GetAIController self) "/Game/AI/CleaningnRobot/BB_CleaningBot.BB_CleaningBot")
  (AI|Components|Blackboard|SetValueasVector _returnvalue (Variables|Default|GetStartLocation) (Transformation|GetActorLocation (Pawn|GetControlledPawn)))
  (AI|Components|Blackboard|SetValueasVector _returnvalue (Variables|Default|GetDestinationLocation) "-500.000000,-100.000000, 0")
  (AI|RunBehaviorTree "/Game/AI/CleaningnRobot/BT_CleaningnBot.BT_CleaningnBot")
  (EventDispatchers|BindEventtoChangedDestinationDispatcher (delegate Custom|Changed%20Destination)))

(fn ConstructionScript)