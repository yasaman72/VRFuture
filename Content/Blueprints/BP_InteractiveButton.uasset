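; BP_InteractiveButton is a physical push button that an overlapping component presses down, calling the Pressed dispatcher at full depth.
; It records the first overlapping component's start location, then each Tick converts its movement into ButtonRoot space to set a clamped press depth along Z.
; When that component leaves, the button interpolates back to rest.
; A DoOnce limits Pressed to one call until the computed depth drops below maximum.
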(event OnComponentBeginOverlap(Button)
  (params (OverlappedComponent :type Primitive%20Component%20Object%20Reference) (OtherActor :type Actor%20Object%20Reference) (OtherComp :type Primitive%20Component%20Object%20Reference) (OtherBodyIndex :type Integer) (bFromSweep :type Boolean) (SweepResult :type Hit%20Result%20Structure%20%28by%20ref%29))
  ;[1 1 1] Detecting other component begin and end overlap
  (Utilities|IsValid (Variables|Default|GetOverlappedComponent)
    (:Is%20Not%20Valid
      (bind _output_get (Variables|Default|SetOverlappedComponent OtherComp))
      (Variables|Default|SetInitialOverlapLocation (Transformation|GetWorldLocation _output_get)))))

(event OnComponentEndOverlap(Button)
  (params (OverlappedComponent :type Primitive%20Component%20Object%20Reference) (OtherActor :type Actor%20Object%20Reference) (OtherComp :type Primitive%20Component%20Object%20Reference) (OtherBodyIndex :type Integer))
  ;[1 1 1] Detecting other component begin and end overlap
  (if (== OtherComp (Variables|Default|GetOverlappedComponent))
    (Variables|Default|SetOverlappedComponent 0)))

(event EventTick
  (params (DeltaSeconds :type Float%20%28single-precision%29))
  (bind _buttonroot (Variables|Default|GetButtonRoot))
  (bind _returnvalue (Transformation|GetWorldTransform _buttonroot))
  (Utilities|FlowControl|Sequence
    (:then_0
      ;[1 1 1] Pressing movement
      (Utilities|IsValid (Variables|Default|GetOverlappedComponent)
        (:Is%20Valid
          (bind _output_get (Variables|Default|SetButtonPressAmount (Math|Float|Clamp(Float) (.z (- (Math|Transform|InverseTransformLocation _returnvalue (Variables|Default|GetInitialOverlapLocation)) (Math|Transform|InverseTransformLocation _returnvalue (Transformation|GetWorldLocation (Variables|Default|GetOverlappedComponent))))) 0.0 (Variables|Default|GetMaxButtonPressAmount))))
          (Transformation|SetRelativeLocation (Variables|Default|GetButton) (Math|Vector|MakeVector 0.0 0.0 (* _output_get -1.0)) false false))
        (:Is%20Not%20Valid
          ;[1 1 1] Depressing the button
          (Transformation|SetRelativeLocation (Variables|Default|GetButton) (Math|Interpolation|VInterpTo (Variables|/Script/Engine.SceneComponent|GetRelativeLocation (Variables|Default|GetButton)) "0, 0, 0" DeltaSeconds 1e+01) false false))))
    (:then_1
      ;[1 1 1] Check button fully pressed
      (if (== (Variables|Default|GetMaxButtonPressAmount) (Variables|Default|GetButtonPressAmount))
        (Utilities|FlowControl|DoOnce false :!label _label
          (:Completed
            (Default|CallPressed)))
        (else
          (goto _label Reset))))))

(fn ConstructionScript)