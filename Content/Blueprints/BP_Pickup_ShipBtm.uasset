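; Bottom half of a two-piece ship pickup that turns into a complete ship when joined to its matching top piece.
; Two socket colliders match their top counterparts by component name and share one attached flag.
; The second match spawns BP_CompleteShip at this mesh's transform and destroys both pieces.
; Any end overlap on either socket clears the flag, whichever component left.
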(event OnComponentBeginOverlap(Socket1BCollider)
  (params (OverlappedComponent :type Primitive%20Component%20Object%20Reference) (OtherActor :type Actor%20Object%20Reference) (OtherComp :type Primitive%20Component%20Object%20Reference) (OtherBodyIndex :type Integer) (bFromSweep :type Boolean) (SweepResult :type Hit%20Result%20Structure%20%28by%20ref%29))
  (if (Utilities|Enum|Equal(Enum) (Utilities|GetObjectName OtherComp) "Socket1TCollider")
    (if (Variables|Default|GetOneIsAttached)
      (Variables|Default|SetOtherActor OtherActor)
      (Game|SpawnActorfromClass "/Game/Blueprints/BP_CompleteShip.BP_CompleteShip_C" (Transformation|GetWorldTransform (Variables|Default|GetStaticMeshComponent)) "Undefined" 0 0)
      (Actor|DestroyActor)
      (Actor|DestroyActor (Variables|Default|GetOtherActor))
      (else
        (Variables|Default|SetOneIsAttached true)))))

(event OnComponentBeginOverlap(Socket2BCollider)
  (params (OverlappedComponent :type Primitive%20Component%20Object%20Reference) (OtherActor :type Actor%20Object%20Reference) (OtherComp :type Primitive%20Component%20Object%20Reference) (OtherBodyIndex :type Integer) (bFromSweep :type Boolean) (SweepResult :type Hit%20Result%20Structure%20%28by%20ref%29))
  (if (Utilities|Enum|Equal(Enum) (Utilities|GetObjectName OtherComp) "Socket2TCollider")
    (if (Variables|Default|GetOneIsAttached)
      (Variables|Default|SetOtherActor OtherActor)
      (Game|SpawnActorfromClass "/Game/Blueprints/BP_CompleteShip.BP_CompleteShip_C" (Transformation|GetWorldTransform (Variables|Default|GetStaticMeshComponent)) "Undefined" 0 0)
      (Actor|DestroyActor)
      (Actor|DestroyActor (Variables|Default|GetOtherActor))
      (else
        (Variables|Default|SetOneIsAttached true)))))

(event OnComponentEndOverlap(Socket2BCollider)
  (params (OverlappedComponent :type Primitive%20Component%20Object%20Reference) (OtherActor :type Actor%20Object%20Reference) (OtherComp :type Primitive%20Component%20Object%20Reference) (OtherBodyIndex :type Integer))
  (Variables|Default|SetOneIsAttached false))

(event OnComponentEndOverlap(Socket1BCollider)
  (params (OverlappedComponent :type Primitive%20Component%20Object%20Reference) (OtherActor :type Actor%20Object%20Reference) (OtherComp :type Primitive%20Component%20Object%20Reference) (OtherBodyIndex :type Integer))
  (Variables|Default|SetOneIsAttached false))

(event EventBeginPlay
  (|CallParentFunction) ; This node is disabled and will not be called.\nDrag off pins to build functionality.
)

(event Collision|EventActorBeginOverlap
  (params (OtherActor :type Actor%20Object%20Reference))
  (|CallParentFunction OtherActor) ; This node is disabled and will not be called.\nDrag off pins to build functionality.
)

(event EventTick
  (params (DeltaSeconds :type Float%20%28single-precision%29)))

(fn ConstructionScript
  (|CallParentFunction))