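; BP_Door is a door that swings on a physics constraint with a configurable angular limit.
; The construction script sets the Swing1 limit and yaws both the constraint and the door mesh by an initial hinge rotation.
; BeginPlay then resets only the door to zero world rotation, leaving the constraint's yaw offset in place.
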(event EventBeginPlay
  (Transformation|SetWorldRotation (Variables|Default|GetDoor) "0, 0, 0" false false))

(event Collision|EventActorBeginOverlap
  (params (OtherActor :type Actor%20Object%20Reference)))

(event EventTick
  (params (DeltaSeconds :type Float%20%28single-precision%29)))

(fn ConstructionScript
  (bind _initialhingerotatio (Variables|Default|GetInitialHingeRotatio))
  (Class|PhysicsConstraintComponent|SetAngularSwing1Limit (Variables|Default|GetPhysicsConstraint) "ACM_Limited" (Variables|Default|GetSwingLimitDgree))
  (Transformation|AddLocalRotation (Variables|Default|GetPhysicsConstraint) (Math|Rotator|MakeRotator 0.0 0.0 _initialhingerotatio) false false)
  (Transformation|AddLocalRotation (Variables|Default|GetDoor) (Math|Rotator|MakeRotator 0.0 0.0 _initialhingerotatio) false false))