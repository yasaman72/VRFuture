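; Gravity gun pickup, held via BP_MotionController, that switches anti-gravity on objects it hits.
; ShootGun or the O key plays a sound, shows a cone and box-traces forward for an actor with an AntiGravityComponent.
; Hit actors lose gravity and drift with random rotation through timeline lerps, or regain gravity if already floating.
; BP_CleaningBot has its own branch that toggles capsule physics, with a delay before physics switches off on restore.
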(event EventShootGun
  ;[1 1 1] Sound
  (Components|Activation|SetActive (Variables|Default|Getphaser2_Cue) true false)
  ;[1 1 1] Cone visibility
  (Rendering|SetVisibility (Variables|Default|GetShape_Cone) true false)
  ;[1 1 1] Gravity state changing
  (bind _hitactor (|LineTracingGravityG))
  (Variables|Default|SetEffectedActor _hitactor)
  (if (Utilities|IsValid (Actor|GetComponentbyClass (Variables|Default|GetEffectedActor) "/Game/Blueprints/Components/AntiGravityComponent.AntiGravityComponent_C"))
    (Variables|Default|SetAntiGravityComponent (Actor|GetComponentbyClass (Variables|Default|GetEffectedActor) "/Game/Blueprints/Components/AntiGravityComponent.AntiGravityComponent_C"))
    (Utilities|Casting|CastToBP_CleaningBot (Variables|Default|GetEffectedActor)
      (:then
        (|ChangeGravityStateBot))
      (:CastFailed
        (|ChangeGravityStateOther)))))

(event EventStoppedShooting
  ;[1 1 1] Sound
  (Audio|Components|Audio|FadeOut (Variables|Default|Getphaser2_Cue) 0.5 0.0 :!class /Script/Engine.AudioComponent)
  ;[1 1 1] Cone visibility
  (Rendering|SetVisibility (Variables|Default|GetShape_Cone) false false))

(event EventPickup
  (params (AttachTo :type Scene%20Component%20Object%20Reference))
  ;[1 1 1] Pick up
  (Physics|SetSimulatePhysics (Variables|Debug|GetStaticMeshComponent) false)
  (Transformation|AttachComponentToComponent (VehicleSound|GetRootComponent) AttachTo "None" "SnapToTarget" "SnapToTarget" "KeepWorld" false)
  (Transformation|SetRelativeLocationAndRotation (Variables|Debug|GetStaticMeshComponent) "-4.200000,-2.000000,-1.700000" "0.000000,-90.000000,4.000000" false true)
  (Variables|Default|SetIsHoldingGun true))

(event EventDrop
  ;[1 1 1] Drop
  (Physics|SetSimulatePhysics (Variables|Debug|GetStaticMeshComponent) false)
  (Transformation|DetachFromActor "KeepWorld" "KeepWorld" "KeepWorld")
  (Variables|Default|SetIsHoldingGun false)
  ;[1 1 1] Sound
  (Audio|Components|Audio|FadeOut (Variables|Default|Getphaser2_Cue) 0.5 0.0 :!class /Script/Engine.AudioComponent)
  ;[1 1 1] Cone visibility
  (Rendering|SetVisibility (Variables|Default|GetShape_Cone) false false))

(event EventBeginPlay
  ;[1 1 1] Begin play
  (Input|EnableInput (Game|GetPlayerController 0))
  (Components|Activation|SetActive (Variables|Default|Getphaser2_Cue) false false)
  (Rendering|SetVisibility (Variables|Default|GetShape_Cone) false false)
  (CallFunction|PrintonWall "Gravity gun text"))

(event Input|KeyboardEvents|O
  (params (Key :type Key%20Structure))
  (bind _phaser2_cue (Variables|Default|Getphaser2_Cue))
  (bind _shape_cone (Variables|Default|GetShape_Cone))
  (:Pressed
    ;[1 1 1] Sound
    (Components|Activation|SetActive _phaser2_cue true false)
    ;[1 1 1] Cone visibility
    (Rendering|SetVisibility _shape_cone true false)
    ;[1 1 1] Gravity state changing
    (bind _hitactor (|LineTracingGravityG))
    (Variables|Default|SetEffectedActor _hitactor)
    (if (Utilities|IsValid (Actor|GetComponentbyClass (Variables|Default|GetEffectedActor) "/Game/Blueprints/Components/AntiGravityComponent.AntiGravityComponent_C"))
      (Variables|Default|SetAntiGravityComponent (Actor|GetComponentbyClass (Variables|Default|GetEffectedActor) "/Game/Blueprints/Components/AntiGravityComponent.AntiGravityComponent_C"))
      (Utilities|Casting|CastToBP_CleaningBot (Variables|Default|GetEffectedActor)
        (:then
          (|ChangeGravityStateBot))
        (:CastFailed
          (|ChangeGravityStateOther)))))
  (:Released
    (Audio|Components|Audio|FadeOut _phaser2_cue 0.5 0.0 :!class /Script/Engine.AudioComponent)
    (Rendering|SetVisibility _shape_cone false false)))

(fn ConstructionScript)

(fn SetHitActorMaterial
  (params (Object :type Object%20Object%20Reference) (self2 :type Primitive%20Component%20Object%20Reference))
  (if (LocalVariables|GetEnteredTheHit)
    _
    (else
      (LocalVariables|SetNewLocalVar_0 (Rendering|Material|GetMaterial self2 0))))
  (if (Utilities|IsValid Object)
    (Rendering|Material|SetMaterial self2 0 "/Game/Material/M_GunRange_2.M_GunRange_2")
    (if (not (LocalVariables|GetEnteredTheHit))
      (LocalVariables|SetEnteredTheHit true))))

(fn PrintonWall
  (params (NewParam :type String))
  (Rendering|Components|TextRender|SetText (Variables|/Script/Engine.TextRenderActor|GetTextRender (Variables|Default|GettextRenderer)) (Utilities|Text|ToText(String) NewParam)))