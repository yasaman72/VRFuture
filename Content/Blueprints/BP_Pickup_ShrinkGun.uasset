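; Motion-controller pickup shrink gun that resizes actors carrying a ScaleablesComponent between small, normal and large.
; Shooting shows the cone, plays sound and box-traces forward, then ChangeSize lerps the hit actor's scale on a timeline toward that component's preset for the current ShrinkState.
; Overlapping the knob while held cycles the state and rotates it; R and S keys also trigger firing and cycling.
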(event OnComponentBeginOverlap(StatePointer)
  (params (OverlappedComponent :type Primitive%20Component%20Object%20Reference) (OtherActor :type Actor%20Object%20Reference) (OtherComp :type Primitive%20Component%20Object%20Reference) (OtherBodyIndex :type Integer) (bFromSweep :type Boolean) (SweepResult :type Hit%20Result%20Structure%20%28by%20ref%29))
  (bind _statepointer (Variables|Default|GetStatePointer))
  (bind _returnvalue (Transformation|GetWorldRotation _statepointer))
  ;[1 1 1] Switch state
  (if (Variables|Default|GetIsHoldingGun)
    (Audio|Components|Audio|Play (Variables|Default|GetbuttonSound) 0.0)
    (if (<= (|GetNumEnumEntries) (Math|Conversions|ToInteger(Byte) (+ (Variables|Default|GetShrinkState) 1)))
      (Variables|Default|SetShrinkState "NewEnumerator0")
      (else
        (Variables|Default|SetShrinkState (Utilities|Enum|ByteToEnumEnum_ShrinkState (+ (Variables|Default|GetShrinkState) 1)))))
    ;[1 1 1] Rotate Knob
    (Transformation|SetWorldLocationAndRotation (Variables|Default|GetStatePointer) (Transformation|GetWorldLocation _statepointer) (Math|Rotator|MakeRotator (+ (.roll _returnvalue) 1.2e+02) (+ (.pitch _returnvalue) 0.0) (+ (.yaw _returnvalue) 0.0)) false false)))

(event EventShootGun
  ;[1 1 1] Sound
  (Components|Activation|SetActive (Variables|Default|Getphaser_Cue) true false)
  ;[1 1 1] Cone visibility
  (Rendering|SetVisibility (Variables|Default|GetShape_Cone) true false)
  ;[1 1 1] Size Changing
  (bind _hitactor (|LineTracingShrtinkG))
  (Variables|Default|SetEffectedActor _hitactor)
  (if (Utilities|IsValid (Actor|GetComponentbyClass (Variables|Default|GetEffectedActor) "/Game/Blueprints/Components/ScaleablesComponent.ScaleablesComponent_C"))
    (|ChangeSize)))

(event EventStoppedShooting
  ;[1 1 1] Sound
  (Audio|Components|Audio|FadeOut (Variables|Default|Getphaser_Cue) 0.5 0.0 :!class /Script/Engine.AudioComponent)
  ;[1 1 1] Cone visibility
  (Rendering|SetVisibility (Variables|Default|GetShape_Cone) false false))

(event EventPickup
  (params (AttachTo :type Scene%20Component%20Object%20Reference))
  ;[1 1 1] Pick up
  (Physics|SetSimulatePhysics (Variables|Debug|GetStaticMeshComponent) false)
  (Transformation|AttachComponentToComponent (VehicleSound|GetRootComponent) AttachTo "None" "SnapToTarget" "SnapToTarget" "KeepWorld" false)
  (Transformation|SetRelativeLocationAndRotation (Variables|Debug|GetStaticMeshComponent) "4.500000,1.000000,1.500000" "0,-90.000000,0.000000" false true)
  (Variables|Default|SetIsHoldingGun true))

(event EventDrop
  ;[1 1 1] Drop
  (Physics|SetSimulatePhysics (Variables|Debug|GetStaticMeshComponent) true)
  (Transformation|DetachFromActor "KeepWorld" "KeepWorld" "KeepWorld")
  (Variables|Default|SetIsHoldingGun false)
  ;[1 1 1] Sound
  (Audio|Components|Audio|FadeOut (Variables|Default|Getphaser_Cue) 0.5 0.0 :!class /Script/Engine.AudioComponent)
  ;[1 1 1] Cone visibility
  (Rendering|SetVisibility (Variables|Default|GetShape_Cone) false false))

(event EventBeginPlay
  ;[1 1 1] Begin play
  (Input|EnableInput (Game|GetPlayerController 0))
  (Components|Activation|SetActive (Variables|Default|Getphaser_Cue) false false)
  (Rendering|SetVisibility (Variables|Default|GetShape_Cone) false false)
  (CallFunction|PrintonWall "Shrinkgun Text")
  (Variables|Default|SetShrinkState "NewEnumerator0"))

(event Input|KeyboardEvents|S
  (params (Key :type Key%20Structure))
  (bind _statepointer (Variables|Default|GetStatePointer))
  (bind _returnvalue (Transformation|GetWorldRotation _statepointer))
  ;[1 1 1] Switch state
  (:Pressed
    (Audio|Components|Audio|Play (Variables|Default|GetbuttonSound) 0.0)
    (if (<= (|GetNumEnumEntries) (Math|Conversions|ToInteger(Byte) (+ (Variables|Default|GetShrinkState) 1)))
      (Variables|Default|SetShrinkState "NewEnumerator0")
      (else
        (Variables|Default|SetShrinkState (Utilities|Enum|ByteToEnumEnum_ShrinkState (+ (Variables|Default|GetShrinkState) 1)))))
    ;[1 1 1] Rotate Knob
    (Transformation|SetWorldLocationAndRotation (Variables|Default|GetStatePointer) (Transformation|GetWorldLocation _statepointer) (Math|Rotator|MakeRotator (+ (.roll _returnvalue) 1.2e+02) (+ (.pitch _returnvalue) 0.0) (+ (.yaw _returnvalue) 0.0)) false false)))

(event Input|KeyboardEvents|R
  (params (Key :type Key%20Structure))
  (bind _phaser_cue (Variables|Default|Getphaser_Cue))
  (bind _shape_cone (Variables|Default|GetShape_Cone))
  (:Pressed
    ;[1 1 1] Sound
    (Components|Activation|SetActive _phaser_cue true false)
    ;[1 1 1] Cone visibility
    (Rendering|SetVisibility _shape_cone true false)
    ;[1 1 1] Size Changing
    (bind _hitactor (|LineTracingShrtinkG))
    (Variables|Default|SetEffectedActor _hitactor)
    (if (Utilities|IsValid (Actor|GetComponentbyClass (Variables|Default|GetEffectedActor) "/Game/Blueprints/Components/ScaleablesComponent.ScaleablesComponent_C"))
      (|ChangeSize)))
  (:Released
    (Audio|Components|Audio|FadeOut _phaser_cue 0.5 0.0 :!class /Script/Engine.AudioComponent)
    (Rendering|SetVisibility _shape_cone false false)))

(fn ConstructionScript)

(fn SetHitActorMaterial
  (params (Object :type Object%20Object%20Reference) (self2 :type Primitive%20Component%20Object%20Reference))
  (if (LocalVariables|GetEnteredTheHit)
    _
    (else
      (LocalVariables|SetNewLocalVar_0 (Rendering|Material|GetMaterial self2 0))))
  (if (Utilities|IsValid Object)
    (Rendering|Material|SetMaterial self2 0 "/Game/Material/M_GunRange_2.M_GunRange_2")
    (if (not (LocalVariables|GetEnteredTheHit))
      (LocalVariables|SetEnteredTheHit true))))

(fn PrintonWall
  (params (textToshow :type String))
  (Rendering|Components|TextRender|SetText (Variables|/Script/Engine.TextRenderActor|GetTextRender (Variables|Default|GetTextRenderer)) (Utilities|Text|ToText(String) textToshow)))