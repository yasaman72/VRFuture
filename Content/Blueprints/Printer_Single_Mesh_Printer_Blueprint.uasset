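; 3D printer actor that spawns a selected printable (plane top, plane bottom or Jax) at its printing origin.
; Three physical buttons, bound on BeginPlay, cycle the object, print it and cycle among three colors; F also prints.
; A dynamic screen material previews the object and a cube shows the color.
; Prints take the class of referenced actors and get rescaled, with the chosen color applied only to Jax.
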(event Custom|Pressed%20Button%201
  ;[1 1 1] Pressing Up Button - Change selected object
  (Development|PrintString "btn 1")
  (if (>= (Utilities|Enum|ByteToEnumEnum_Printables (+ (Variables|Default|GetPrintables) 1)) (Math|Conversions|ToByte(Integer) (|GetNumEnumEntries)))
    (Variables|Default|SetPrintables "NewEnumerator0")
    (else
      (Variables|Default|SetPrintables (Utilities|Enum|ByteToEnumEnum_Printables (+ (Variables|Default|GetPrintables) 1)))))
  (bind _returnvalue (Rendering|Material|CreateDynamicMaterialInstance (Variables|Default|GetPrinterUVScreen) 2 "/Game/Shaders/JetsonsTV.JetsonsTV" "None" :!class /Script/Engine.PrimitiveComponent))
  (switch Utilities|FlowControl|Switch|SwitchonEnum_Printables (Variables|Default|GetPrintables)
    (:NewEnumerator0
      (Rendering|Material|SetTextureParameterValue _returnvalue "ScreenImage" "/Game/Shaders/SpaceShip_Top.SpaceShip_Top"))
    (:NewEnumerator1
      (Rendering|Material|SetTextureParameterValue _returnvalue "ScreenImage" "/Game/Shaders/SpaceShip_Bottom.SpaceShip_Bottom"))
    (:NewEnumerator2
      (Rendering|Material|SetTextureParameterValue _returnvalue "ScreenImage" "/Game/Shaders/Jax.Jax"))))

(event Custom|Pressed%20Button%202
  (bind _printing_origin (Variables|Default|GetPrinting_origin))
  (bind _returnvalue (Transformation|GetWorldLocation _printing_origin))
  (bind _returnvalue_2 (Math|Conversions|ToTransform(Vector) _returnvalue))
  ;[1 1 1] Printing Something
  (Development|PrintString "btn 2")
  (switch Utilities|FlowControl|Switch|SwitchonEnum_Printables (Variables|Default|GetPrintables)
    (:NewEnumerator0
      (bind _returnvalue_3 (Game|SpawnActorfromClass (Utilities|GetClass (Variables|Default|GetGenerating%20Actor0)) _returnvalue_2 "Undefined" 0 0))
      (Transformation|SetActorScale3D _returnvalue_3 "0.700000,0.700000,0.700000"))
    (:NewEnumerator1
      (bind _returnvalue_4 (Game|SpawnActorfromClass (Utilities|GetClass (Variables|Default|GetGenerating%20Actor1)) _returnvalue_2 "Undefined" 0 0))
      (Transformation|SetActorScale3D _returnvalue_4 "0.700000,0.700000,0.700000"))
    (:NewEnumerator2
      (bind _returnvalue_5 (Game|SpawnActorfromClass (Utilities|GetClass (Variables|Default|GetGenerating%20Actor2)) _returnvalue_2 "Undefined" 0 0))
      (Transformation|SetActorScale3D _returnvalue_5 "0.500000,0.500000,0.500000")
      (switch Utilities|FlowControl|Switch|SwitchonEnum_Color (Variables|Default|GetPrintColor)
        (:NewEnumerator0
          (Rendering|Material|SetVectorParameterValueonMaterials (Actor|GetComponentbyClass _returnvalue_5 "/Script/Engine.StaticMeshComponent") "Color" (Math|Conversions|ToVector(LinearColor) "(R=0.971354,G=0.690418,B=0.000000,A=1.000000)")))
        (:NewEnumerator1
          (Rendering|Material|SetVectorParameterValueonMaterials (Actor|GetComponentbyClass _returnvalue_5 "/Script/Engine.StaticMeshComponent") "Color" (Math|Conversions|ToVector(LinearColor) "(R=0.721354,G=0.024421,B=0.706960,A=1.000000)")))
        (:NewEnumerator2
          (Rendering|Material|SetVectorParameterValueonMaterials (Actor|GetComponentbyClass _returnvalue_5 "/Script/Engine.StaticMeshComponent") "Color" (Math|Conversions|ToVector(LinearColor) "(R=0.029867,G=0.955729,B=0.102931,A=1.000000)")))))))

(event Custom|Pressed%20Button%203
  (bind _cube (Variables|Default|GetCube))
  ;[1 1 1] Change selected Color
  (Development|PrintString "Btn 3")
  (if (>= (Utilities|Enum|ByteToEnumEnum_Color (+ (Variables|Default|GetPrintColor) 1)) (Math|Conversions|ToByte(Integer) (|GetNumEnumEntries)))
    (Variables|Default|SetPrintColor "NewEnumerator0")
    (else
      (Variables|Default|SetPrintColor (Utilities|Enum|ByteToEnumEnum_Color (+ (Variables|Default|GetPrintColor) 1)))))
  (switch Utilities|FlowControl|Switch|SwitchonEnum_Color (Variables|Default|GetPrintColor)
    (:NewEnumerator0
      (Rendering|Material|SetVectorParameterValueonMaterials _cube "Color" (Math|Conversions|ToVector(LinearColor) "(R=0.971354,G=0.690418,B=0.000000,A=1.000000)")))
    (:NewEnumerator1
      (Rendering|Material|SetVectorParameterValueonMaterials _cube "Color" (Math|Conversions|ToVector(LinearColor) "(R=0.721354,G=0.024421,B=0.706960,A=1.000000)")))
    (:NewEnumerator2
      (Rendering|Material|SetVectorParameterValueonMaterials _cube "Color" (Math|Conversions|ToVector(LinearColor) "(R=0.029867,G=0.955729,B=0.102931,A=1.000000)")))))

(event EventBeginPlay
  (Input|EnableInput (Game|GetPlayerController 0))
  ;[1 1 1] Initial Visual
  (bind _returnvalue (Rendering|Material|CreateDynamicMaterialInstance (Variables|Default|GetPrinterUVScreen) 2 "/Game/Shaders/JetsonsTV.JetsonsTV" "None" :!class /Script/Engine.PrimitiveComponent))
  (Rendering|Material|SetTextureParameterValue _returnvalue "ScreenImage" "/Game/Shaders/SpaceShip_Top.SpaceShip_Top")
  (Rendering|Material|SetVectorParameterValueonMaterials (Variables|Default|GetCube) "Color" (Math|Conversions|ToVector(LinearColor) "(R=0.971354,G=0.690418,B=0.000000,A=1.000000)"))
  ;[1 1 1] Binding to button press events
  (EventDispatchers|BindEventtoPressed (Variables|Default|GetPhysical%20Button%201) (delegate Custom|Pressed%20Button%201))
  (EventDispatchers|BindEventtoPressed (Variables|Default|GetPhysical%20Button%202) (delegate Custom|Pressed%20Button%202))
  (EventDispatchers|BindEventtoPressed (Variables|Default|GetPhysical%20Button%203) (delegate Custom|Pressed%20Button%203)))

(event Input|KeyboardEvents|F
  (params (Key :type Key%20Structure))
  (bind _printing_origin (Variables|Default|GetPrinting_origin))
  (bind _returnvalue (Transformation|GetWorldLocation _printing_origin))
  (bind _returnvalue_2 (Math|Conversions|ToTransform(Vector) _returnvalue))
  ;[1 1 1] Printing Something
  (:Pressed
    (switch Utilities|FlowControl|Switch|SwitchonEnum_Printables (Variables|Default|GetPrintables)
      (:NewEnumerator0
        (bind _returnvalue_3 (Game|SpawnActorfromClass (Utilities|GetClass (Variables|Default|GetGenerating%20Actor0)) _returnvalue_2 "Undefined" 0 0))
        (Transformation|SetActorScale3D _returnvalue_3 "0.700000,0.700000,0.700000"))
      (:NewEnumerator1
        (bind _returnvalue_4 (Game|SpawnActorfromClass (Utilities|GetClass (Variables|Default|GetGenerating%20Actor1)) _returnvalue_2 "Undefined" 0 0))
        (Transformation|SetActorScale3D _returnvalue_4 "0.700000,0.700000,0.700000"))
      (:NewEnumerator2
        (bind _returnvalue_5 (Game|SpawnActorfromClass (Utilities|GetClass (Variables|Default|GetGenerating%20Actor2)) _returnvalue_2 "Undefined" 0 0))
        (Transformation|SetActorScale3D _returnvalue_5 "0.500000,0.500000,0.500000")
        (switch Utilities|FlowControl|Switch|SwitchonEnum_Color (Variables|Default|GetPrintColor)
          (:NewEnumerator0
            (Rendering|Material|SetVectorParameterValueonMaterials (Actor|GetComponentbyClass _returnvalue_5 "/Script/Engine.StaticMeshComponent") "Color" (Math|Conversions|ToVector(LinearColor) "(R=0.971354,G=0.690418,B=0.000000,A=1.000000)")))
          (:NewEnumerator1
            (Rendering|Material|SetVectorParameterValueonMaterials (Actor|GetComponentbyClass _returnvalue_5 "/Script/Engine.StaticMeshComponent") "Color" (Math|Conversions|ToVector(LinearColor) "(R=0.721354,G=0.024421,B=0.706960,A=1.000000)")))
          (:NewEnumerator2
            (Rendering|Material|SetVectorParameterValueonMaterials (Actor|GetComponentbyClass _returnvalue_5 "/Script/Engine.StaticMeshComponent") "Color" (Math|Conversions|ToVector(LinearColor) "(R=0.029867,G=0.955729,B=0.102931,A=1.000000)"))))))))

(fn ConstructionScript)