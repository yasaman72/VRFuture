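; Actor component that plays a random impact sound when its owner's static mesh hits something.
; One second after BeginPlay it binds to the mesh's hit event.
; Hits play when velocity times mass exceeds MinImpact times mass, effectively a speed threshold, spawning a Sounds entry at the owner's location at Volume.
; A DoOnce reset after MinSoundInterval throttles repeats; the random index range includes the array length, one past the last entry.
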(event Custom|OnComponentHit_Event_0
  (params (HitComponent :type Primitive%20Component%20Object%20Reference) (OtherActor :type Actor%20Object%20Reference) (OtherComp :type Primitive%20Component%20Object%20Reference) (NormalImpulse :type Vector) (Hit :type Hit%20Result%20Structure%20%28by%20ref%29))
  (bind _returnvalue (Components|GetOwner))
  (bind _sounds (Variables|Default|GetSounds))
  (bind _returnvalue_2 (Actor|GetComponentbyClass _returnvalue "/Script/Engine.PrimitiveComponent"))
  (bind _returnvalue_3 (Physics|GetMass _returnvalue_2))
  (if (> (* (Math|Vector|VectorLength (Transformation|GetVelocity _returnvalue)) _returnvalue_3) (* _returnvalue_3 (Variables|Default|GetMinImpact)))
    (Utilities|FlowControl|DoOnce false :!label _label
      (:Completed
        (Audio|SpawnSoundatLocation (Utilities|Array|Get(acopy) _sounds (Math|Random|RandomIntegerinRange 0 (Utilities|Array|Length _sounds))) (Transformation|GetActorLocation (Components|GetOwner)) "0, 0, 0" (Variables|Default|GetVolume) 1.0 0.0 0 0)
        (Utilities|FlowControl|Delay (Variables|Default|GetMinSoundInterval))
        (goto _label Reset)))))

(event EventBeginPlay
  (Utilities|FlowControl|Delay 1.0)
  (Collision|AssignOnComponentHit (Actor|GetComponentbyClass (Components|GetOwner) "/Script/Engine.StaticMeshComponent") (delegate Custom|OnComponentHit_Event_0)))