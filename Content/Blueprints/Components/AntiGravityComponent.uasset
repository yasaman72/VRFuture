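; An actor component meant to give its owner anti-gravity, though the effect is unfinished.
; On BeginPlay it takes the owner's first static mesh component, enables physics simulation and sets gravity from InitialGravity.
; ToggleGravity only flips the IsAntiGravity flag.
; AntiGravityFunction is empty, with disconnected nodes that would disable gravity and raise the mesh.
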(event Custom|ToggleGravity
  (if (Variables|Default|GetIsAntiGravity)
    (Variables|Default|SetIsAntiGravity false)
    (else
      (Variables|Default|SetIsAntiGravity true))))

(event EventBeginPlay
  (bind _output_get (Variables|Default|SetPrimitiveComponent (Utilities|Array|Get(acopy) (Actor|GetComponentsByClass (Components|GetOwner) "/Script/Engine.StaticMeshComponent"))))
  (Physics|SetSimulatePhysics _output_get true)
  (Physics|SetEnableGravity _output_get (Variables|Default|GetInitialGravity)))

(fn AntiGravityFunction)