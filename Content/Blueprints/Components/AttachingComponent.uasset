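; Actor component meant to snap a designated AttachableActor onto its owner when the two meet.
; On BeginPlay it searches the owner's attached actors for a TriggerBox and stores it.
; An overlap handler attaches the matching actor's root to the owner's root at the AttachToThis socket, keeping world scale.
; The node binding that handler to the trigger box is unconnected, so the attachment never fires as written.
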(event Custom|OnActorBeginOverlap_Event_0
  (params (OverlappedActor :type Actor%20Object%20Reference) (OtherActor :type Actor%20Object%20Reference))
  (if (== OtherActor (Variables|Default|GetAttachableActor))
    (Development|PrintString "found my mate!")
    (Transformation|AttachComponentToComponent (Variables|/Script/Engine.Actor|GetRootComponent OtherActor) (Variables|/Script/Engine.Actor|GetRootComponent (Components|GetOwner)) "AttachToThis" "SnapToTarget" "SnapToTarget" "KeepWorld" true)))

(event EventBeginPlay
  ;[1 1 1] Getting owner trigger box
  (for _array_element (Actor|GetAttachedActors (Components|GetOwner))
    (if (Utilities|ClassIsChildOf (Utilities|GetClass _array_element) "/Script/Engine.TriggerBox")
      (bind _astrigger_box (Utilities|Casting|CastToTriggerBox _array_element))
      (Variables|Default|SetTriggerBox _astrigger_box))))