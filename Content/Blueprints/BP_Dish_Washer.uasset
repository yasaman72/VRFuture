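; Dish washer with a conveyor that carries objects along and destroys plates reaching its trigger box.
; ConveyorBox stores one overlapping physics-simulating actor, ignoring player-tagged actors such as hands, and clears it on any end overlap.
; Tick offsets that actor along the Arrow's forward vector at Speed, without sweep, while it has no attached actors.
; TriggerBox destroys Plate-tagged actors whose overlapping component is simulating physics.
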(event OnComponentBeginOverlap(TriggerBox)
  (params (OverlappedComponent :type Primitive%20Component%20Object%20Reference) (OtherActor :type Actor%20Object%20Reference) (OtherComp :type Primitive%20Component%20Object%20Reference) (OtherBodyIndex :type Integer) (bFromSweep :type Boolean) (SweepResult :type Hit%20Result%20Structure%20%28by%20ref%29))
  ;[0.6458 1 0.994] Destroy Plates
  (if (Actor|ActorHasTag OtherActor "Plate")
    (if (Physics|IsSimulatingPhysics OtherComp "None")
      (Actor|DestroyActor OtherActor))))

(event OnComponentBeginOverlap(ConveyorBox)
  (params (OverlappedComponent :type Primitive%20Component%20Object%20Reference) (OtherActor :type Actor%20Object%20Reference) (OtherComp :type Primitive%20Component%20Object%20Reference) (OtherBodyIndex :type Integer) (bFromSweep :type Boolean) (SweepResult :type Hit%20Result%20Structure%20%28by%20ref%29))
  ;[0.4177 0.4177 0.4177] Move and stop moving - Check to make sure its not a hand!
  (if (not (Actor|ActorHasTag OtherActor "PlayerTag"))
    (if (Physics|IsSimulatingPhysics OtherComp "None")
      (Variables|Default|SetActorToMove OtherActor))))

(event OnComponentEndOverlap(ConveyorBox)
  (params (OverlappedComponent :type Primitive%20Component%20Object%20Reference) (OtherActor :type Actor%20Object%20Reference) (OtherComp :type Primitive%20Component%20Object%20Reference) (OtherBodyIndex :type Integer))
  ;[0.4177 0.4177 0.4177] Move and stop moving - Check to make sure its not a hand!
  (Variables|Default|SetActorToMove 0))

(event EventTick
  (params (DeltaSeconds :type Float%20%28single-precision%29))
  (bind _actortomove (Variables|Default|GetActorToMove))
  ;[1 1 1] Move on tick
  (if (Utilities|IsValid _actortomove)
    (if (== (Utilities|Array|Length (Actor|GetAttachedActors _actortomove)) 0)
      (Transformation|AddActorWorldOffset _actortomove (* (* (Math|Vector|GetForwardVector (Variables|Default|GetArrow)) (Variables|Default|GetSpeed)) DeltaSeconds)))))

(fn ConstructionScript)