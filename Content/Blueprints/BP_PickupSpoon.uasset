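; A spoon actor that BP_MotionController can pick up and drop.
; Pickup turns off physics on the static mesh and attaches the root to the given component, keeping its world transform; Drop re-enables physics and detaches it.
; Any overlap on the mesh swaps its material to a shrink-triggered one, and ending an overlap restores the initial material, with no shrinking logic in this Blueprint.
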(event OnComponentBeginOverlap(StaticMeshComponent)
  (params (OverlappedComponent :type Primitive%20Component%20Object%20Reference) (OtherActor :type Actor%20Object%20Reference) (OtherComp :type Primitive%20Component%20Object%20Reference) (OtherBodyIndex :type Integer) (bFromSweep :type Boolean) (SweepResult :type Hit%20Result%20Structure%20%28by%20ref%29))
  (Rendering|Material|SetMaterial (Variables|Debug|GetStaticMeshComponent) 0 (Variables|Default|GetShrinkTriggeredMaterial)))

(event OnComponentEndOverlap(StaticMeshComponent)
  (params (OverlappedComponent :type Primitive%20Component%20Object%20Reference) (OtherActor :type Actor%20Object%20Reference) (OtherComp :type Primitive%20Component%20Object%20Reference) (OtherBodyIndex :type Integer))
  (Rendering|Material|SetMaterial (Variables|Debug|GetStaticMeshComponent) 0 (Variables|Default|GetInitialMaterial)))

(event EventBeginPlay)

(event Collision|EventActorBeginOverlap
  (params (OtherActor :type Actor%20Object%20Reference)))

(event EventPickup
  (params (AttachTo :type Scene%20Component%20Object%20Reference))
  (Physics|SetSimulatePhysics (Variables|Debug|GetStaticMeshComponent) false)
  (Transformation|AttachComponentToComponent (VehicleSound|GetRootComponent) AttachTo "None" "KeepWorld" "KeepWorld" "KeepWorld" false))

(event EventDrop
  (Physics|SetSimulatePhysics (Variables|Debug|GetStaticMeshComponent) true)
  (Transformation|DetachFromActor "KeepWorld" "KeepWorld" "KeepWorld"))

(fn ConstructionScript)