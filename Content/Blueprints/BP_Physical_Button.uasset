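; BP_Physical_Button is a pressable button built from a Button component, a physics constraint and a press collision volume.
; The construction script offsets the constraint by the button's relative location and locks angular swing 2, deriving its angle from button pitch.
; Any overlap with the press volume fires the pressed event dispatcher, while the debug message prints only when the Button itself overlaps.
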(event OnComponentBeginOverlap(ButtonPressCollision)
  (params (OverlappedComponent :type Primitive%20Component%20Object%20Reference) (OtherActor :type Actor%20Object%20Reference) (OtherComp :type Primitive%20Component%20Object%20Reference) (OtherBodyIndex :type Integer) (bFromSweep :type Boolean) (SweepResult :type Hit%20Result%20Structure%20%28by%20ref%29))
  (Default|CallPressedButtonEventDispatcher)
  (if (== OtherComp (Variables|Default|GetButton))
    (Development|PrintString "Pressed the button")))

(fn ConstructionScript
  (bind _physicsconstraint (Variables|Default|GetPhysicsConstraint))
  (bind _button (Variables|Default|GetButton))
  (Class|PhysicsConstraintComponent|SetAngularSwing2Limit _physicsconstraint "ACM_Locked" (+ (.Pitch (Math|Rotator|BreakRotator (Variables|/Script/Engine.SceneComponent|GetRelativeRotation _button))) 1.8e+02))
  (Transformation|AddLocalOffset _physicsconstraint (Variables|/Script/Engine.SceneComponent|GetRelativeLocation _button) false false))

(fn PressedButton
  (return false false))