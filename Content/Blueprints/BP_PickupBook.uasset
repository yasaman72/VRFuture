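; BP_PickupBook is a physics book prop that BP_MotionController can grab and drop.
; Pickup turns off physics and attaches the actor to the given component, while Drop re-enables physics and detaches it, both keeping world transform.
; The construction script randomizes the mesh scale and picks one of four book meshes for variety.
; Overlapping the mesh swaps its material to a shrink-triggered one and restores the initial material when overlap ends.
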(event OnComponentBeginOverlap(StaticMeshComponent)
  (params (OverlappedComponent :type Primitive%20Component%20Object%20Reference) (OtherActor :type Actor%20Object%20Reference) (OtherComp :type Primitive%20Component%20Object%20Reference) (OtherBodyIndex :type Integer) (bFromSweep :type Boolean) (SweepResult :type Hit%20Result%20Structure%20%28by%20ref%29))
  (Rendering|Material|SetMaterial (Variables|Debug|GetStaticMeshComponent) 0 (Variables|Default|GetShrinkTriggeredMaterial)))

(event OnComponentEndOverlap(StaticMeshComponent)
  (params (OverlappedComponent :type Primitive%20Component%20Object%20Reference) (OtherActor :type Actor%20Object%20Reference) (OtherComp :type Primitive%20Component%20Object%20Reference) (OtherBodyIndex :type Integer))
  (Rendering|Material|SetMaterial (Variables|Debug|GetStaticMeshComponent) 0 (Variables|Default|GetInitialMaterial)))

(event EventBeginPlay)

(event Collision|EventActorBeginOverlap
  (params (OtherActor :type Actor%20Object%20Reference)))

(event EventPickup
  (params (AttachTo :type Scene%20Component%20Object%20Reference))
  (Physics|SetSimulatePhysics (Variables|Debug|GetStaticMeshComponent) false)
  (Transformation|AttachComponentToComponent (VehicleSound|GetRootComponent) AttachTo "None" "KeepWorld" "KeepWorld" "KeepWorld" false))

(event EventDrop
  (Physics|SetSimulatePhysics (Variables|Debug|GetStaticMeshComponent) true)
  (Transformation|DetachFromActor "KeepWorld" "KeepWorld" "KeepWorld"))

(fn ConstructionScript
  (bind _staticmeshcomponent (Variables|Debug|GetStaticMeshComponent))
  (Transformation|SetRelativeScale3D (Variables|Debug|GetStaticMeshComponent) (Math|Vector|MakeVector (Math|Random|RandomFloatinRange 0.8 1.3) (Math|Random|RandomFloatinRange 0.8 1.3) (Math|Random|RandomFloatinRange 0.95 1.05)))
  (switch int (Math|Random|RandomIntegerinRange 0 3)
    (:0
      (Components|StaticMesh|SetStaticMesh _staticmeshcomponent "/Game/Models/Books_Plane_004.Books_Plane_004"))
    (:1
      (Components|StaticMesh|SetStaticMesh _staticmeshcomponent "/Game/Models/Books_Plane_005.Books_Plane_005"))
    (:2
      (Components|StaticMesh|SetStaticMesh _staticmeshcomponent "/Game/Models/Books_Plane_006.Books_Plane_006"))
    (:3
      (Components|StaticMesh|SetStaticMesh _staticmeshcomponent "/Game/Models/Books_Plane_009.Books_Plane_009"))))