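; BP_Radio is a physics prop radio that motion controllers can pick up and drop, with a turnable dial for switching channels.
; It plays an introduction sound on BeginPlay, then starts the first channel and calls FinishedIntroductionMessage if IsPlayingTutorial was set.
; Outside the tutorial, key 1 or a knob overlap plays a click and advances a MultiGate through three channels and off, rotating the dial to match.
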(event OnComponentBeginOverlap(KnobCol)
  (params (OverlappedComponent :type Primitive%20Component%20Object%20Reference) (OtherActor :type Actor%20Object%20Reference) (OtherComp :type Primitive%20Component%20Object%20Reference) (OtherBodyIndex :type Integer) (bFromSweep :type Boolean) (SweepResult :type Hit%20Result%20Structure%20%28by%20ref%29))
  (bind _btnsndplayer (Variables|Default|GetBtnSndPlayer))
  ;[1 1 1] Switch state
  (if (not (Variables|Default|GetIsPlayingTutorial))
    (Audio|Components|Audio|SetSound _btnsndplayer (Variables|Default|GetBtnSound))
    (Audio|Components|Audio|Play _btnsndplayer 0.0)
    (Utilities|FlowControl|MultiGate false false -1
      (:Out%200
        (Audio|Components|Audio|SetSound (Variables|Default|GetAudioPlayer) (Utilities|Array|Get(acopy) (Variables|Default|GetChannelsSounds)))
        (Transformation|SetRelativeRotation (Variables|Default|GetRadioWithDial_Radio_Dial) "0, 0, 0" false false)
        (Audio|Components|Audio|Play (Variables|Default|GetAudioPlayer) 0.0 :!label _label))
      (:Out%201
        (Audio|Components|Audio|SetSound (Variables|Default|GetAudioPlayer) (Utilities|Array|Get(acopy) (Variables|Default|GetChannelsSounds) 1))
        (Transformation|SetRelativeRotation (Variables|Default|GetRadioWithDial_Radio_Dial) "45.000000, 0, 0" false false)
        (goto _label))
      (:Out%202
        (Audio|Components|Audio|SetSound (Variables|Default|GetAudioPlayer) (Utilities|Array|Get(acopy) (Variables|Default|GetChannelsSounds) 2))
        (Transformation|SetRelativeRotation (Variables|Default|GetRadioWithDial_Radio_Dial) "90.000000, 0, 0" false false)
        (goto _label))
      (:Out%203
        (Audio|Components|Audio|Stop (Variables|Default|GetAudioPlayer))
        (Transformation|SetRelativeRotation (Variables|Default|GetRadioWithDial_Radio_Dial) "130.000000, 0, 0" false false)
        (CallFunction|ResetMultiGate)))))

(event OnAudioFinished(AudioPlayer)
  ;[1 1 1] Control introduction play
  (if (Variables|Default|GetIsPlayingTutorial)
    (Variables|Default|SetIsPlayingTutorial false)
    (CallFunction|PlayRadio)
    (Class|HintVoicesInterface|FinishedIntroduction(Message))))

(event Custom|ResetMultiGate
  ;[1 1 1] Switch state
  (Utilities|FlowControl|MultiGate false false -1) ; enters at Reset
)

(event Custom|PlayRadio
  ;[1 1 1] Switch state
  (Utilities|FlowControl|MultiGate false false -1
    (:Out%200
      (Audio|Components|Audio|SetSound (Variables|Default|GetAudioPlayer) (Utilities|Array|Get(acopy) (Variables|Default|GetChannelsSounds)))
      (Transformation|SetRelativeRotation (Variables|Default|GetRadioWithDial_Radio_Dial) "0, 0, 0" false false)
      (Audio|Components|Audio|Play (Variables|Default|GetAudioPlayer) 0.0 :!label _label))
    (:Out%201
      (Audio|Components|Audio|SetSound (Variables|Default|GetAudioPlayer) (Utilities|Array|Get(acopy) (Variables|Default|GetChannelsSounds) 1))
      (Transformation|SetRelativeRotation (Variables|Default|GetRadioWithDial_Radio_Dial) "45.000000, 0, 0" false false)
      (goto _label))
    (:Out%202
      (Audio|Components|Audio|SetSound (Variables|Default|GetAudioPlayer) (Utilities|Array|Get(acopy) (Variables|Default|GetChannelsSounds) 2))
      (Transformation|SetRelativeRotation (Variables|Default|GetRadioWithDial_Radio_Dial) "90.000000, 0, 0" false false)
      (goto _label))
    (:Out%203
      (Audio|Components|Audio|Stop (Variables|Default|GetAudioPlayer))
      (Transformation|SetRelativeRotation (Variables|Default|GetRadioWithDial_Radio_Dial) "130.000000, 0, 0" false false)
      (CallFunction|ResetMultiGate))))

(event EventPickup
  (params (AttachTo :type Scene%20Component%20Object%20Reference))
  (bind _staticmeshcomponent (Variables|Debug|GetStaticMeshComponent))
  ;[1 1 1] Pickup
  (Physics|SetSimulatePhysics _staticmeshcomponent false)
  (Transformation|AttachComponentToComponent _staticmeshcomponent AttachTo "None" "KeepWorld" "KeepWorld" "KeepWorld" false))

(event EventBeginPlay
  (bind _audioplayer (Variables|Default|GetAudioPlayer))
  ;[1 1 1] Begin Play
  (Audio|Components|Audio|SetSound _audioplayer (Variables|Default|GetIntroductionSound))
  (Audio|Components|Audio|Play _audioplayer 0.0))

(event EventDrop
  ;[1 1 1] Drop
  (Physics|SetSimulatePhysics (Variables|Debug|GetStaticMeshComponent) true)
  (Transformation|DetachFromActor "KeepWorld" "KeepWorld" "KeepWorld"))

(event Input|KeyboardEvents|1
  (params (Key :type Key%20Structure))
  (bind _btnsndplayer (Variables|Default|GetBtnSndPlayer))
  ;[1 1 1] Switch state
  (:Pressed
    (if (not (Variables|Default|GetIsPlayingTutorial))
      (Audio|Components|Audio|SetSound _btnsndplayer (Variables|Default|GetBtnSound))
      (Audio|Components|Audio|Play _btnsndplayer 0.0)
      (Utilities|FlowControl|MultiGate false false -1
        (:Out%200
          (Audio|Components|Audio|SetSound (Variables|Default|GetAudioPlayer) (Utilities|Array|Get(acopy) (Variables|Default|GetChannelsSounds)))
          (Transformation|SetRelativeRotation (Variables|Default|GetRadioWithDial_Radio_Dial) "0, 0, 0" false false)
          (Audio|Components|Audio|Play (Variables|Default|GetAudioPlayer) 0.0 :!label _label))
        (:Out%201
          (Audio|Components|Audio|SetSound (Variables|Default|GetAudioPlayer) (Utilities|Array|Get(acopy) (Variables|Default|GetChannelsSounds) 1))
          (Transformation|SetRelativeRotation (Variables|Default|GetRadioWithDial_Radio_Dial) "45.000000, 0, 0" false false)
          (goto _label))
        (:Out%202
          (Audio|Components|Audio|SetSound (Variables|Default|GetAudioPlayer) (Utilities|Array|Get(acopy) (Variables|Default|GetChannelsSounds) 2))
          (Transformation|SetRelativeRotation (Variables|Default|GetRadioWithDial_Radio_Dial) "90.000000, 0, 0" false false)
          (goto _label))
        (:Out%203
          (Audio|Components|Audio|Stop (Variables|Default|GetAudioPlayer))
          (Transformation|SetRelativeRotation (Variables|Default|GetRadioWithDial_Radio_Dial) "130.000000, 0, 0" false false)
          (CallFunction|ResetMultiGate))))))

(fn ConstructionScript)