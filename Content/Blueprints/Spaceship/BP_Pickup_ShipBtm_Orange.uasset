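; Orange bottom-half ship pickup that merges with a top half into a complete ship when both sockets line up.
; Two socket colliders match top-socket colliders by name, sharing one flag so the second match triggers assembly.
; Assembly spawns BP_CompleteShip with both halves' meshes, passes it to the holding hand and destroys both pickups.
; A separate event, uncalled here, caches the top half's holding hand through casts.
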(event OnComponentBeginOverlap(Socket1BCollider)
  (params (OverlappedComponent :type Primitive%20Component%20Object%20Reference) (OtherActor :type Actor%20Object%20Reference) (OtherComp :type Primitive%20Component%20Object%20Reference) (OtherBodyIndex :type Integer) (bFromSweep :type Boolean) (SweepResult :type Hit%20Result%20Structure%20%28by%20ref%29))
  (bind _holdinghand (Variables|Default|GetHoldingHand))
  (if (Utilities|Enum|Equal(Enum) (Utilities|GetObjectName OtherComp) "Socket1TCollider")
    (if (Variables|Default|GetOneIsAttached)
      (Variables|Default|SetOtherActor OtherActor)
      (bind _returnvalue (Game|SpawnActorfromClass "/Game/Blueprints/Spaceship/BP_CompleteShip.BP_CompleteShip_C" (Transformation|GetWorldTransform (Variables|Default|GetStaticMeshComponent)) "Undefined" 0 0))
      (Variables|/Game/Blueprints/Spaceship/BP_CompleteShip.BP_CompleteShip_C|SetTopStaticMesh _returnvalue (Variables|/Script/Engine.StaticMeshComponent|GetStaticMesh (Actor|GetComponentbyClass (Variables|Default|GetOtherActor) "/Script/Engine.StaticMeshComponent")))
      (Variables|/Game/Blueprints/Spaceship/BP_CompleteShip.BP_CompleteShip_C|SetDownStaticMesh _returnvalue (Variables|/Script/Engine.StaticMeshComponent|GetStaticMesh (Variables|Default|GetStaticMeshComponent)))
      (if (Utilities|IsValid _holdinghand)
        (Default|Pickup _returnvalue _holdinghand))
      (if (Utilities|IsValid (Variables|Default|GetOtherActor))
        (Class|PickupActorInterface|Drop(Message) (Variables|Default|GetOtherActor)))
      (Actor|DestroyActor)
      (Actor|DestroyActor (Variables|Default|GetOtherActor))
      (else
        (Variables|Default|SetOneIsAttached true)))))

(event OnComponentBeginOverlap(Socket2BCollider)
  (params (OverlappedComponent :type Primitive%20Component%20Object%20Reference) (OtherActor :type Actor%20Object%20Reference) (OtherComp :type Primitive%20Component%20Object%20Reference) (OtherBodyIndex :type Integer) (bFromSweep :type Boolean) (SweepResult :type Hit%20Result%20Structure%20%28by%20ref%29))
  (bind _holdinghand (Variables|Default|GetHoldingHand))
  (if (Utilities|Enum|Equal(Enum) (Utilities|GetObjectName OtherComp) "Socket2TCollider")
    (if (Variables|Default|GetOneIsAttached)
      (Variables|Default|SetOtherActor OtherActor)
      (bind _returnvalue (Game|SpawnActorfromClass "/Game/Blueprints/Spaceship/BP_CompleteShip.BP_CompleteShip_C" (Transformation|GetWorldTransform (Variables|Default|GetStaticMeshComponent)) "Undefined" 0 0))
      (Variables|/Game/Blueprints/Spaceship/BP_CompleteShip.BP_CompleteShip_C|SetTopStaticMesh _returnvalue (Variables|/Script/Engine.StaticMeshComponent|GetStaticMesh (Actor|GetComponentbyClass (Variables|Default|GetOtherActor) "/Script/Engine.StaticMeshComponent")))
      (Variables|/Game/Blueprints/Spaceship/BP_CompleteShip.BP_CompleteShip_C|SetDownStaticMesh _returnvalue (Variables|/Script/Engine.StaticMeshComponent|GetStaticMesh (Variables|Default|GetStaticMeshComponent)))
      (if (Utilities|IsValid _holdinghand)
        (Default|Pickup _returnvalue _holdinghand))
      (if (Utilities|IsValid (Variables|Default|GetOtherActor))
        (Class|PickupActorInterface|Drop(Message) (Variables|Default|GetOtherActor)))
      (Actor|DestroyActor)
      (Actor|DestroyActor (Variables|Default|GetOtherActor))
      (else
        (Variables|Default|SetOneIsAttached true)))))

(event OnComponentEndOverlap(Socket2BCollider)
  (params (OverlappedComponent :type Primitive%20Component%20Object%20Reference) (OtherActor :type Actor%20Object%20Reference) (OtherComp :type Primitive%20Component%20Object%20Reference) (OtherBodyIndex :type Integer))
  (Variables|Default|SetOneIsAttached false))

(event OnComponentEndOverlap(Socket1BCollider)
  (params (OverlappedComponent :type Primitive%20Component%20Object%20Reference) (OtherActor :type Actor%20Object%20Reference) (OtherComp :type Primitive%20Component%20Object%20Reference) (OtherBodyIndex :type Integer))
  (Variables|Default|SetOneIsAttached false))

(event OnComponentBeginOverlap(StaticMeshComponent)
  (params (OverlappedComponent :type Primitive%20Component%20Object%20Reference) (OtherActor :type Actor%20Object%20Reference) (OtherComp :type Primitive%20Component%20Object%20Reference) (OtherBodyIndex :type Integer) (bFromSweep :type Boolean) (SweepResult :type Hit%20Result%20Structure%20%28by%20ref%29)))

(event OnComponentEndOverlap(StaticMeshComponent)
  (params (OverlappedComponent :type Primitive%20Component%20Object%20Reference) (OtherActor :type Actor%20Object%20Reference) (OtherComp :type Primitive%20Component%20Object%20Reference) (OtherBodyIndex :type Integer)))

(event Custom|SetOtherHoldingHand
  (bind _otheractor (Variables|Default|GetOtherActor))
  (bind _asbp_pickup_top_orange (Utilities|Casting|CastToBP_Pickup_Top_Orange _otheractor)
    (:then
      (Variables|Default|SetOtherHoldingHand (Variables|/Game/Blueprints/Spaceship/BP_Pickup_Top_Orange.BP_Pickup_Top_Orange_C|GetHoldingHand _asbp_pickup_top_orange)))
    (:CastFailed
      (bind _asbp_pickup_ship_top_yellow (Utilities|Casting|CastToBP_Pickup_ShipTop_Yellow _otheractor)
        (:then
          (Variables|Default|SetOtherHoldingHand (Variables|/Game/Blueprints/Spaceship/BP_Pickup_ShipTop_Yellow.BP_Pickup_ShipTop_Yellow_C|GetHoldingHand _asbp_pickup_ship_top_yellow)))
        (:CastFailed
          (bind _asbp_pickup_ship_top_green (Utilities|Casting|CastToBP_Pickup_ShipTop_Green _otheractor))
          (Variables|Default|SetOtherHoldingHand (Variables|/Game/Blueprints/Spaceship/BP_Pickup_ShipTop_Green.BP_Pickup_ShipTop_Green_C|GetHoldingHand _asbp_pickup_ship_top_green)))))))

(event EventBeginPlay
  (|CallParentFunction) ; This node is disabled and will not be called.\nDrag off pins to build functionality.
)

(event EventTick
  (params (DeltaSeconds :type Float%20%28single-precision%29)))

(fn ConstructionScript
  (|CallParentFunction))