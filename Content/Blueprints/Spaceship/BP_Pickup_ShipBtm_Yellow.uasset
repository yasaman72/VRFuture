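; Pickup actor for the yellow bottom half of a spaceship, which merges with a top half to form a complete ship.
; Its two socket colliders look for the matching top colliders by component name, sharing one flag so the second match triggers assembly.
; Assembly spawns BP_CompleteShip at the bottom mesh's transform, copies both meshes onto it, passes it to any holding hand and destroys both halves.
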(event OnComponentBeginOverlap(Socket1BCollider)
  (params (OverlappedComponent :type Primitive%20Component%20Object%20Reference) (OtherActor :type Actor%20Object%20Reference) (OtherComp :type Primitive%20Component%20Object%20Reference) (OtherBodyIndex :type Integer) (bFromSweep :type Boolean) (SweepResult :type Hit%20Result%20Structure%20%28by%20ref%29))
  (bind _holdinghand (Variables|Default|GetHoldingHand))
  (if (Utilities|Enum|Equal(Enum) (Utilities|GetObjectName OtherComp) "Socket1TCollider")
    (if (Variables|Default|GetOneIsAttached)
      (Variables|Default|SetOtherActor OtherActor)
      (bind _returnvalue (Game|SpawnActorfromClass "/Game/Blueprints/Spaceship/BP_CompleteShip.BP_CompleteShip_C" (Transformation|GetWorldTransform (Variables|Default|GetStaticMeshComponent)) "Undefined" 0 0))
      (Variables|/Game/Blueprints/Spaceship/BP_CompleteShip.BP_CompleteShip_C|SetTopStaticMesh _returnvalue (Variables|/Script/Engine.StaticMeshComponent|GetStaticMesh (Actor|GetComponentbyClass (Variables|Default|GetOtherActor) "/Script/Engine.StaticMeshComponent")))
      (Variables|/Game/Blueprints/Spaceship/BP_CompleteShip.BP_CompleteShip_C|SetDownStaticMesh _returnvalue (Variables|/Script/Engine.StaticMeshComponent|GetStaticMesh (Variables|Default|GetStaticMeshComponent)))
      (if (Utilities|IsValid _holdinghand)
        (Default|Pickup _returnvalue _holdinghand))
      (Actor|DestroyActor (Variables|Default|GetOtherActor))
      (Actor|DestroyActor)
      (else
        (Variables|Default|SetOneIsAttached true)))))

(event OnComponentBeginOverlap(Socket2BCollider)
  (params (OverlappedComponent :type Primitive%20Component%20Object%20Reference) (OtherActor :type Actor%20Object%20Reference) (OtherComp :type Primitive%20Component%20Object%20Reference) (OtherBodyIndex :type Integer) (bFromSweep :type Boolean) (SweepResult :type Hit%20Result%20Structure%20%28by%20ref%29))
  (bind _holdinghand (Variables|Default|GetHoldingHand))
  (if (Utilities|Enum|Equal(Enum) (Utilities|GetObjectName OtherComp) "Socket2TCollider")
    (if (Variables|Default|GetOneIsAttached)
      (Variables|Default|SetOtherActor OtherActor)
      (bind _returnvalue (Game|SpawnActorfromClass "/Game/Blueprints/Spaceship/BP_CompleteShip.BP_CompleteShip_C" (Transformation|GetWorldTransform (Variables|Default|GetStaticMeshComponent)) "Undefined" 0 0))
      (Variables|/Game/Blueprints/Spaceship/BP_CompleteShip.BP_CompleteShip_C|SetTopStaticMesh _returnvalue (Variables|/Script/Engine.StaticMeshComponent|GetStaticMesh (Actor|GetComponentbyClass (Variables|Default|GetOtherActor) "/Script/Engine.StaticMeshComponent")))
      (Variables|/Game/Blueprints/Spaceship/BP_CompleteShip.BP_CompleteShip_C|SetDownStaticMesh _returnvalue (Variables|/Script/Engine.StaticMeshComponent|GetStaticMesh (Variables|Default|GetStaticMeshComponent)))
      (if (Utilities|IsValid _holdinghand)
        (Default|Pickup _returnvalue _holdinghand))
      (Actor|DestroyActor (Variables|Default|GetOtherActor))
      (Actor|DestroyActor)
      (else
        (Variables|Default|SetOneIsAttached true)))))

(event OnComponentEndOverlap(Socket2BCollider)
  (params (OverlappedComponent :type Primitive%20Component%20Object%20Reference) (OtherActor :type Actor%20Object%20Reference) (OtherComp :type Primitive%20Component%20Object%20Reference) (OtherBodyIndex :type Integer))
  (Variables|Default|SetOneIsAttached false))

(event OnComponentEndOverlap(Socket1BCollider)
  (params (OverlappedComponent :type Primitive%20Component%20Object%20Reference) (OtherActor :type Actor%20Object%20Reference) (OtherComp :type Primitive%20Component%20Object%20Reference) (OtherBodyIndex :type Integer))
  (Variables|Default|SetOneIsAttached false))

(event OnComponentBeginOverlap(StaticMeshComponent)
  (params (OverlappedComponent :type Primitive%20Component%20Object%20Reference) (OtherActor :type Actor%20Object%20Reference) (OtherComp :type Primitive%20Component%20Object%20Reference) (OtherBodyIndex :type Integer) (bFromSweep :type Boolean) (SweepResult :type Hit%20Result%20Structure%20%28by%20ref%29)))

(event OnComponentEndOverlap(StaticMeshComponent)
  (params (OverlappedComponent :type Primitive%20Component%20Object%20Reference) (OtherActor :type Actor%20Object%20Reference) (OtherComp :type Primitive%20Component%20Object%20Reference) (OtherBodyIndex :type Integer)))

(event EventBeginPlay
  (|CallParentFunction) ; This node is disabled and will not be called.\nDrag off pins to build functionality.
)

(event EventTick
  (params (DeltaSeconds :type Float%20%28single-precision%29)))

(fn ConstructionScript
  (|CallParentFunction))