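; BP_CompleteShip is a spaceship Blueprint that displays a ship built from a top and a bottom static mesh.
; On the first Tick, a DoOnce assigns TopStaticMesh and DownStaticMesh to its two mesh components.
; BeginPlay and the construction script only call the parent versions, and the component overlap events are empty.
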(event OnComponentBeginOverlap(StaticMeshComponent)
  (params (OverlappedComponent :type Primitive%20Component%20Object%20Reference) (OtherActor :type Actor%20Object%20Reference) (OtherComp :type Primitive%20Component%20Object%20Reference) (OtherBodyIndex :type Integer) (bFromSweep :type Boolean) (SweepResult :type Hit%20Result%20Structure%20%28by%20ref%29)))

(event OnComponentEndOverlap(StaticMeshComponent)
  (params (OverlappedComponent :type Primitive%20Component%20Object%20Reference) (OtherActor :type Actor%20Object%20Reference) (OtherComp :type Primitive%20Component%20Object%20Reference) (OtherBodyIndex :type Integer)))

(event EventBeginPlay
  (|CallParentFunction))

(event EventTick
  (params (DeltaSeconds :type Float%20%28single-precision%29))
  (Utilities|FlowControl|DoOnce false
    (:Completed
      (Components|StaticMesh|SetStaticMesh (Variables|Default|GetStaticMeshComponent) (Variables|Default|GetTopStaticMesh))
      (Components|StaticMesh|SetStaticMesh (Variables|Default|GetStaticMeshBtm) (Variables|Default|GetDownStaticMesh)))))

(fn ConstructionScript
  (|CallParentFunction))